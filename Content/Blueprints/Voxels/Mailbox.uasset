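; Mailbox is a Blueprint, filed under Voxels, that accrues a dollar balance on a repeating timer and shows it on a floating widget.
; Each Tick turns the widget component to face the player camera and counts a cooldown down from RewardTimeSeconds.
; When the cooldown runs out, it carries the remainder into the next cycle, adds DollarsPerReward to CurrentBalance and writes the total into the WBP_MailboxBalance widget.
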(event `self.ReceiveBeginPlay`
  (set `self.Cooldown` (`self.RewardTimeSeconds`)))

(event `self.ReceiveTick`
  (params (DeltaSeconds :type "Float (single-precision)"))
  (`|ExecutionSequence`
    (:`then_0`
      (`SceneComponent.K2_SetWorldRotation` (`self.Widget`) (`KismetMathLibrary.Conv_VectorToRotator` (- (`PlayerCameraManager.GetCameraLocation` (`GameplayStatics.GetPlayerCameraManager` 0)) (`SceneComponent.K2_GetComponentLocation` (`self.Widget`)))) false false))
    (:`then_1`
      (bind _output_get (set `self.Cooldown` (- (`self.Cooldown`) DeltaSeconds)))
      (if (<= _output_get 0.0)
        (set `self.Cooldown` (+ (`self.Cooldown`) (`self.RewardTimeSeconds`)))
        (set `self.CurrentBalance` (+ (`self.CurrentBalance`) (`self.DollarsPerReward`)))
        (bind _aswbp_mailbox_balance (cast `/Game/Blueprints/UI/World/WBP_MailboxBalance` (`WidgetComponent.GetUserWidgetObject` (`self.Widget`))))
        (set `/Game/Blueprints/UI/World/WBP_MailboxBalance.Balance` (`self.CurrentBalance`) _aswbp_mailbox_balance)))))

(fn `UserConstructionScript`)