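; Voxel transport pipe that adapts its appearance to which of its six sides have active endpoints.
; RefreshMesh decodes the ActiveEndpoints bitmask into per-direction custom primitive data on the Endpoints component, and writes the inverted mask to Center.
; Each float carries the raw masked bit value rather than a normalized 0 or 1, presumably for the material to read.
; GetCardinalDirection maps an index to one of the six directions.
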(fn `GetCardinalDirection`
  (params (Index :type Integer))
  (returns (OutputValue :type "EFGTransportPipeDirections Enum"))
  (return (select `int` Index :`0` "Forward" :`1` "Backward" :`2` "Right" :`3` "Left" :`4` "Up" :`5` "Down" :!type "EFGTransportPipeDirections Enum")))

(fn `RefreshMesh`
  (`|ExecutionSequence`
    (:`then_0`
      ;[1 1 1] Endpoints
      ;;[1 1 1] Forward
      (`PrimitiveComponent.SetDefaultCustomPrimitiveDataFloat` (`self.Endpoints`) 0 (`KismetMathLibrary.Conv_IntToDouble` (`KismetMathLibrary.And_IntInt` (`self.ActiveEndpoints`) 1)))
      ;;[1 1 1] Backward
      (`PrimitiveComponent.SetDefaultCustomPrimitiveDataFloat` (`self.Endpoints`) 1 (`KismetMathLibrary.Conv_IntToDouble` (`KismetMathLibrary.And_IntInt` (`self.ActiveEndpoints`) 2)))
      ;;[1 1 1] Left
      (`PrimitiveComponent.SetDefaultCustomPrimitiveDataFloat` (`self.Endpoints`) 2 (`KismetMathLibrary.Conv_IntToDouble` (`KismetMathLibrary.And_IntInt` (`self.ActiveEndpoints`) 4)))
      ;;[1 1 1] Right
      (`PrimitiveComponent.SetDefaultCustomPrimitiveDataFloat` (`self.Endpoints`) 3 (`KismetMathLibrary.Conv_IntToDouble` (`KismetMathLibrary.And_IntInt` (`self.ActiveEndpoints`) 8)))
      ;;[1 1 1] Up
      (`PrimitiveComponent.SetDefaultCustomPrimitiveDataFloat` (`self.Endpoints`) 4 (`KismetMathLibrary.Conv_IntToDouble` (`KismetMathLibrary.And_IntInt` (`self.ActiveEndpoints`) 16)))
      ;;[1 1 1] Down
      (`PrimitiveComponent.SetDefaultCustomPrimitiveDataFloat` (`self.Endpoints`) 5 (`KismetMathLibrary.Conv_IntToDouble` (`KismetMathLibrary.And_IntInt` (`self.ActiveEndpoints`) 32))))
    (:`then_1`
      ;[1 1 1] Center
      ;;[1 1 1] Forward
      (`PrimitiveComponent.SetDefaultCustomPrimitiveDataFloat` (`self.Center`) 0 (`KismetMathLibrary.Conv_IntToDouble` (`KismetMathLibrary.And_IntInt` (`KismetMathLibrary.Not_Int` (`self.ActiveEndpoints`)) 1)))
      ;;[1 1 1] Backward
      (`PrimitiveComponent.SetDefaultCustomPrimitiveDataFloat` (`self.Center`) 1 (`KismetMathLibrary.Conv_IntToDouble` (`KismetMathLibrary.And_IntInt` (`KismetMathLibrary.Not_Int` (`self.ActiveEndpoints`)) 2)))
      ;;[1 1 1] Left
      (`PrimitiveComponent.SetDefaultCustomPrimitiveDataFloat` (`self.Center`) 2 (`KismetMathLibrary.Conv_IntToDouble` (`KismetMathLibrary.And_IntInt` (`KismetMathLibrary.Not_Int` (`self.ActiveEndpoints`)) 4)))
      ;;[1 1 1] Right
      (`PrimitiveComponent.SetDefaultCustomPrimitiveDataFloat` (`self.Center`) 3 (`KismetMathLibrary.Conv_IntToDouble` (`KismetMathLibrary.And_IntInt` (`KismetMathLibrary.Not_Int` (`self.ActiveEndpoints`)) 8)))
      ;;[1 1 1] Up
      (`PrimitiveComponent.SetDefaultCustomPrimitiveDataFloat` (`self.Center`) 4 (`KismetMathLibrary.Conv_IntToDouble` (`KismetMathLibrary.And_IntInt` (`KismetMathLibrary.Not_Int` (`self.ActiveEndpoints`)) 16)))
      ;;[1 1 1] Down
      (`PrimitiveComponent.SetDefaultCustomPrimitiveDataFloat` (`self.Center`) 5 (`KismetMathLibrary.Conv_IntToDouble` (`KismetMathLibrary.And_IntInt` (`KismetMathLibrary.Not_Int` (`self.ActiveEndpoints`)) 32))))))

(fn `UserConstructionScript`)